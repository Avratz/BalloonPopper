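; LoopsGameMode is a game mode that procedurally spawns a pyramid of Box actors on BeginPlay.
; BuildPyramid loops over levels, passing a shrinking side length to BuildBase, which uses nested loops to place boxes on a square grid through SpawnBox.
; Each level rises by a fixed height, and its X and Y positions are divided by the level number plus one, compressing upper layers toward the world origin.
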(event EventBeginPlay
  (CallFunction|BuildPyramid 4))

(fn ConstructionScript)

(fn BuildBase
  (params (X :type Integer) (Y :type Integer) (Level :type Integer))
  (bind _returnvalue (+ Level 1))
  (for _index (range 0 X)
    (for _index_2 (range 0 Y)
      (CallFunction|SpawnBox (/ (+ (+ (Math|Vector|MakeVector 0.0 0.0 (* (Math|Conversions|ToFloat(Integer) Level) 1.5e+02)) (* _index "100.000000,0.000000,0.000000")) (* _index_2 "0.000000,100.000000,0.000000")) (Math|Vector|MakeVector (Math|Conversions|ToFloat(Integer) _returnvalue) (Math|Conversions|ToFloat(Integer) _returnvalue) 1.0))))))

(fn SpawnBox
  (params (Location :type Vector))
  (Game|SpawnActorfromClass "/Game/Loops/Blueprints/Box.Box_C" (Math|Transform|MakeTransform Location) "Undefined" "MultiplyWithRoot" 0 0))

(fn BuildPyramid
  (params (Base :type Integer))
  (for _index (range 0 Base)
    (CallFunction|BuildBase (- Base _index) (- Base _index) _index)))